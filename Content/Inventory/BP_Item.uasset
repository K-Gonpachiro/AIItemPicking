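; BP_Item is an item actor that shows a widget while the third-person character is within its collision sphere.
; Sphere overlap events toggle the widget and invert the AI sight stimulus: unregistered while the character overlaps, registered again when they leave.
; Tick moves the widget to follow the sphere mesh in X and Y at a fixed world height.
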(event `self.ReceiveTick`
  (params (DeltaSeconds :type "Float (single-precision)"))
  (bind (_returnvalue_x _returnvalue_y) (`KismetMathLibrary.BreakVector` (`SceneComponent.K2_GetComponentLocation` (`self.SphereMesh`))))
  (`SceneComponent.K2_SetWorldLocation` (`self.Widget`) (`KismetMathLibrary.MakeVector` _returnvalue_x _returnvalue_y 150.0) false false))

(event `self.SphereCollision.OnComponentBeginOverlap`
  (params (OverlappedComponent :type "PrimitiveComponent Object Reference") (OtherActor :type "Actor Object Reference") (OtherComp :type "PrimitiveComponent Object Reference") (OtherBodyIndex :type Integer) (bFromSweep :type Boolean) (SweepResult :type "HitResult Structure (by ref)"))
  (cast `/Game/ThirdPerson/Blueprints/BP_ThirdPersonCharacter` OtherActor)
  (`SceneComponent.SetVisibility` (`self.Widget`) true false)
  (`AIPerceptionStimuliSourceComponent.UnregisterFromSense` (`self.AIPerceptionStimuliSource`) "/Script/AIModule.AISense_Sight"))

(event `self.SphereCollision.OnComponentEndOverlap`
  (params (OverlappedComponent :type "PrimitiveComponent Object Reference") (OtherActor :type "Actor Object Reference") (OtherComp :type "PrimitiveComponent Object Reference") (OtherBodyIndex :type Integer))
  (cast `/Game/ThirdPerson/Blueprints/BP_ThirdPersonCharacter` OtherActor)
  (`SceneComponent.SetVisibility` (`self.Widget`) false false)
  (`AIPerceptionStimuliSourceComponent.RegisterForSense` (`self.AIPerceptionStimuliSource`) "/Script/AIModule.AISense_Sight"))

(fn `UserConstructionScript`)