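; BP_SeePoints is an area actor that spawns a grid of BP_Node see points at BeginPlay and stores them in SeePointNodes.
; Spacing on each axis is that spline's length divided by the node count minus one.
; Nodes extend from the root's location along world X and Y, ignoring spline shape and actor rotation.
; CleanArray then walks the array in reverse to remove invalid entries.
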(event `self.ReceiveBeginPlay`
  ;[1 1 1] Spawn Nodes
  (`self.SetXSpacing`)
  (`self.SetYSpacing`)
  (for _index (range 1 (+ (`self.NodesX`) 1))
    (for _index_2 (range 1 (+ (`self.NodesY`) 1))
      (bind _returnvalue (`|SpawnActorFromClass` "/Game/AreaInfo/BP_Node.BP_Node_C" (`KismetMathLibrary.Conv_VectorToTransform` (+ (`SceneComponent.K2_GetComponentLocation` (`self.DefaultSceneRoot`)) (`KismetMathLibrary.MakeVector` (* (- _index 1) (`self.XSpacing`)) (* (- _index_2 1) (`self.YSpacing`))))) "Undefined" "MultiplyWithRoot" null null))
      (`KismetArrayLibrary.Array_Add` (`self.SeePointNodes`) _returnvalue)))
  (`self.CleanArray`))

(event `CleanArray`
  (bind _seepointnodes (`self.SeePointNodes`))
  (bind (_arrayindex _arrayelement) (`/Engine/EditorBlueprintResources/StandardMacros.ReverseForEachLoop` _seepointnodes)
    (:`LoopBody`
      (if (not (`KismetSystemLibrary.IsValid` _arrayelement))
        (`KismetArrayLibrary.Array_Remove` _seepointnodes _arrayindex)))))

(fn `SetXSpacing`
  (set `self.XSpacing` (/ (`SplineComponent.GetSplineLength` (`self.SplineX`)) (- (`self.NodesX`) 1))))

(fn `SetYSpacing`
  (set `self.YSpacing` (/ (`SplineComponent.GetSplineLength` (`self.SplineY`)) (- (`self.NodesY`) 1))))

(fn `UserConstructionScript`)