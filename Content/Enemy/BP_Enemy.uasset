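; Enemy character that spots the player through PawnSensing and reports sighting state to its AI Blackboard.
; On first sight it caches the player, sets hasSeenPlayer and starts a looping timer that traces head to head, updating the last seen location.
; A failed trace clears the flag, stops the timer, rearms detection and sets hasLostPlayer.
; It also forwards item pickup and drop events to a pickup system component.
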(event `self.ReceiveBeginPlay`
  (set `/Game/Inventory/AC_PickupSystem.CapsuleCollision` (`self.CapsuleComponent`) (`self.AC_PickupSystem`)))

(event `self.PawnSensing.OnSeePawn`
  (params (Pawn :type "Pawn Object Reference"))
  (`/Engine/EditorBlueprintResources/StandardMacros.DoOnce` false :!label _label
    (:`Completed`
      (`KismetSystemLibrary.K2_SetTimer` null "CheckPlayerSight" 0.25 true)
      (bind _asbp_third_person_character (cast `/Game/ThirdPerson/Blueprints/BP_ThirdPersonCharacter` Pawn))
      (set `self.BP Third Person Character` _asbp_third_person_character)
      (`self.SetPlayerVisibility` true))))

(event `ResetTimer`
  (goto _label :!via `Reset`))

(event `PickUpItem`
  (`/Game/Inventory/AC_PickupSystem.AddItem` (`self.AC_PickupSystem`)))

(event `DropItem`
  (`/Game/Inventory/AC_PickupSystem.DropItem` (`self.AC_PickupSystem`)))

(fn `CheckPlayerSight`
  (if (`self.hasSeenPlayer`)
    (bind _outhit (`KismetSystemLibrary.LineTraceSingleForObjects` (`SceneComponent.GetSocketLocation` (`self.Mesh`) "Head") (`SceneComponent.GetSocketLocation` (`Character.Mesh` (`self.BP Third Person Character`)) "Head") (`self.LTObjs`)))
    (bind _asbp_third_person_character (cast `/Game/ThirdPerson/Blueprints/BP_ThirdPersonCharacter` (`.HitActor` (`GameplayStatics.BreakHitResult` _outhit)))
      (:`then`
        (set `self.LastSeenLocation` (`self.K2_GetActorLocation` _asbp_third_person_character)))
      (:`CastFailed`
        (`self.SetPlayerVisibility` false)
        (`KismetSystemLibrary.K2_ClearTimer` null "CheckPlayerSight")
        (`self.ResetTimer`)
        (`BlackboardComponent.SetValueAsBool` (`AIBlueprintHelperLibrary.GetBlackboard` (`AIBlueprintHelperLibrary.GetAIController` self)) "hasLostPlayer" true)))))

(fn `SetPlayerVisibility`
  (params (hasSeenPlayer :type Boolean))
  (bind _output_get (set `self.hasSeenPlayer` hasSeenPlayer))
  (`BlackboardComponent.SetValueAsBool` (`AIBlueprintHelperLibrary.GetBlackboard` (`AIBlueprintHelperLibrary.GetAIController` self)) "hasSeenPlayer" _output_get))

(fn `UserConstructionScript`)